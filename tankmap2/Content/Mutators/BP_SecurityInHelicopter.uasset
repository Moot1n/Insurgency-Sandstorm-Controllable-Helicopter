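; Insurgency mutator that starts a human team-0 (Security) player in the driver seat of an airborne helicopter each round.
; It massively enlarges playable areas and removes restricted areas to open up flight.
; Five seconds into each round, it spawns team-tagged helicopters high above objective spawn zones with rotors running.
; It seats the first human team-0 soldier found, then destroys helicopters left without a driver.
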(event `self.OnGameStateInitialized`
  (params (InGameState :type "INSGameState Object Reference"))
  (for _array_element (`INSGameState.PlayableAreas` InGameState) :!label _label
    (bind _brushcomponent (`Brush.BrushComponent` _array_element))
    (`SceneComponent.SetWorldScale3D` _brushcomponent (* (`SceneComponent.K2_GetComponentScale` _brushcomponent) 300.0)))
  (for _array_element_2 (`INSGameState.RestrictedAreas` InGameState)
    (`Actor.K2_DestroyActor` _array_element_2)))

(event `self.InitializeMutator`
  (params (GameMode :type "INSGameMode Object Reference") (Options :type String))
  (goto _label))

(event `self.InitializeMutatorPostLoad`
  (bind _asinsgame_mode (cast `INSGameMode` (`GameplayStatics.GetGameMode`)))
  (set `INSGameMode.bAllowRestrictedAreas` false _asinsgame_mode))

(event `self.OnRoundStarted`
  (bind _spawnedhelis (`self.SpawnedHelis`))
  (for _array_element (`self.SpawnedHelis`)
    (`Actor.K2_DestroyActor` _array_element))
  (`KismetArrayLibrary.Array_Clear` (`self.SpawnedHelis`))
  (`KismetSystemLibrary.Delay` 5.0)
  (bind _asinsgame_mode (cast `INSGameMode` (`GameplayStatics.GetGameMode`)))
  (for _array_element_2 (`INSGameState.Objectives` (`INSGameMode.INSGameState` _asinsgame_mode))
    (for _array_element_3 (`ObjectiveBase.AssociatedSpawnZones` _array_element_2)
      (bind _returnvalue (`|SpawnActorFromClass` "/tankmap/Game/Actors/Vehicles/BP_VH_MyHeli3.BP_VH_MyHeli3_C" (`KismetMathLibrary.Conv_VectorToTransform` (+ (`Actor.K2_GetActorLocation` _array_element_3) (* (`KismetMathLibrary.Vector_Up`) 8000.0))) "DontSpawnIfColliding" "OverrideRootScale" null null))
      (`/Engine/EditorBlueprintResources/StandardMacros.IsValid` _returnvalue
        (:`Is Valid`
          (set `VehicleBase.TeamId` (`SpawnZone.TeamId` _array_element_3) _returnvalue)
          (`KismetArrayLibrary.Array_Add` (`self.SpawnedHelis`) _returnvalue)
          (set `/tankmap/Game/Actors/Vehicles/BP_VH_MyHeli3.rotorSpeed` 1.0 _returnvalue)
          (set `/tankmap/Game/Actors/Vehicles/BP_VH_MyHeli3.rotorSpeedTarget` 1.0 _returnvalue))))
    (for _index (range (+ (`INSFindSessionCallbackProxy.GetCurrentPlayers` (make `BlueprintFindSessionResult`)) 1))
      (bind _returnvalue_2 (`GameplayStatics.GetPlayerPawn` _index))
      (`/Engine/EditorBlueprintResources/StandardMacros.IsValid` _returnvalue_2
        (:`Is Valid`
          (bind _asinssoldier (cast `INSSoldier` _returnvalue_2))
          (cast `INSAISoldierController` (`Pawn.GetController` _asinssoldier)
            (:`CastFailed`
              (if (`Pawn.IsBotControlled` _asinssoldier)
                _
                (elif (== (`INSSoldier.GetTeamId` _asinssoldier) 0)
                  (for _array_element_4 _spawnedhelis
                    (`/Engine/EditorBlueprintResources/StandardMacros.IsValid` _array_element_4
                      (:`Is Valid`
                        (if (== (`VehicleBase.TeamId` _array_element_4) (`INSSoldier.GetTeamId` _asinssoldier))
                          (`VehicleSeatComponent.EnterSeat` (`/tankmap/Game/Actors/Vehicles/BP_VH_MyHeli3.Driver` _array_element_4) _asinssoldier false)
                          (set `/tankmap/Game/Actors/Vehicles/BP_VH_MyHeli3.rotorSpeedTarget` 1.0 _array_element_4)
                          (break)))))
                  (break)))))))))
  (for _array_element_5 _spawnedhelis
    (`/Engine/EditorBlueprintResources/StandardMacros.IsValid` (`VehicleSeatComponent.GetSeatedCharacter` (`/tankmap/Game/Actors/Vehicles/BP_VH_MyHeli3.Driver` _array_element_5))
      (:`Is Not Valid`
        (`Actor.K2_DestroyActor` _array_element_5)))))

(event `self.OnPlayerSpawned`
  (params (Soldier :type "INSSoldier Object Reference") (NewPlayer :type "Controller Object Reference") (StartRotation :type "Rotator Structure (by ref)")))