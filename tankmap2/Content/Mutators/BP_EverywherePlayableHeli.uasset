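; Mutator that opens up the map's playable space in an INSGameMode match by removing restricted areas and enlarging playable areas.
; After load it turns off the game mode's AllowRestrictedAreas flag.
; On the first round start only, it adds the extra width and height variables to each playable area brush's world scale, then destroys every restricted area actor listed in the game state.
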(event `self.OnRoundStarted`
  (if (not (`self.Once`))
    (set `self.Once` true)
    (`self.deleteRestricted`)))

(event `self.InitializeMutatorPostLoad`
  (bind _asinsgame_mode (cast `INSGameMode` (`GameplayStatics.GetGameMode`)))
  (set `INSGameMode.bAllowRestrictedAreas` false _asinsgame_mode))

(event `deleteRestricted`
  (bind _fpaextrawidth (`self.fPAExtraWidth`))
  (bind _asinsgame_mode (cast `INSGameMode` (`GameplayStatics.GetGameMode`)))
  (bind _insgamestate (`INSGameMode.INSGameState` _asinsgame_mode))
  (for _array_element (`INSGameState.PlayableAreas` _insgamestate)
    (bind _brushcomponent (`Brush.BrushComponent` _array_element))
    (`SceneComponent.SetWorldScale3D` _brushcomponent (`KismetMathLibrary.MakeVector` (+ (.x (`SceneComponent.K2_GetComponentScale` _brushcomponent)) _fpaextrawidth) (+ (.y (`SceneComponent.K2_GetComponentScale` _brushcomponent)) _fpaextrawidth) (+ (.z (`SceneComponent.K2_GetComponentScale` _brushcomponent)) (`self.fPAExtraHeight`)))))
  (for _array_element_2 (`INSGameState.RestrictedAreas` _insgamestate)
    (`Actor.K2_DestroyActor` _array_element_2)))