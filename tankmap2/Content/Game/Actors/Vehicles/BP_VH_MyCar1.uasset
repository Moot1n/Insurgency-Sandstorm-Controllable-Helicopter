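; Vehicle Blueprint for a car with a turret-mounted GAU19 gun operated from the TurretGunner seat.
; On BeginPlay, InitMountedGunGameLogic2 spawns the weapon on authority at the turret's pitch socket, sets automatic fire, stores it for replication and runs visual setup.
; InitMountedGunGameLogic is an identical copy that this file never calls.
; The Driver's move-forward delegate only prints a debug string.
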(event `self.ReceiveBeginPlay`
  (`self.InitMountedGunGameLogic2`)
  (add `VehicleSeatComponent.Delegate_OnMoveForward` (`self.Driver`) (delegate `Delegate_OnMoveForward_Event_0`)))

(event `Delegate_OnMoveForward_Event_0`
  (params (InputValue :type "Float (double-precision)"))
  (`KismetSystemLibrary.PrintString` "HelloMovedForward"))

(fn `InitMountedGunGameLogic`
  ;[1 1 1] Comment
  (`/Engine/EditorBlueprintResources/ActorMacros.Switch Has Authority`
    (:`Authority`
      (bind _returnvalue (`WeaponStatics.SpawnMountedWeapon` "/Game/Game/Actors/Weapons/HeavyMachineGun/BP_Firearm_GAU19.BP_Firearm_GAU19_C" self (`self.TurretYaw`) "pitch" (`self.TurretGunner`)))
      (`ItemFirearm.SetFiremode` _returnvalue "Automatic")
      ;;[1 1 1] [Saber Atai] SS-36261- added replication
      (set `self.SpawnedMountedWeapon` _returnvalue)
      (`self.InitMountedGunVisualLogic`))))

(fn `InitMountedGunGameLogic2`
  ;[1 1 1] Comment
  (`/Engine/EditorBlueprintResources/ActorMacros.Switch Has Authority`
    (:`Authority`
      (bind _returnvalue (`WeaponStatics.SpawnMountedWeapon` "/Game/Game/Actors/Weapons/HeavyMachineGun/BP_Firearm_GAU19.BP_Firearm_GAU19_C" self (`self.TurretYaw`) "pitch" (`self.TurretGunner`)))
      (`ItemFirearm.SetFiremode` _returnvalue "Automatic")
      ;;[1 1 1] [Saber Atai] SS-36261- added replication
      (set `self.SpawnedMountedWeapon` _returnvalue)
      (`self.InitMountedGunVisualLogic`))))

(fn `UserConstructionScript`
  (`parent.UserConstructionScript`))