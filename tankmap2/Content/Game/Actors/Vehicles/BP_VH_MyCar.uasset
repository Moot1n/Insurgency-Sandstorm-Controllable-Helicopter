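; Drivable car Blueprint with a mounted rocket turret operated from a gunner seat.
; On BeginPlay the server spawns automatic Apache rockets on the turret yaw's pitch socket, links them to the gunner seat, stores the weapon and initializes gun visuals.
; Seat-entered delegates bind to an empty handler.
; InitMountedGunGameLogic is an uncalled duplicate of the active init function, and a delayed engine-kill snippet is unwired.
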(event `self.ReceiveBeginPlay`
  (`self.InitMountedGunGameLogic2`)
  (add `VehicleSeatComponent.Delegate_OnSeatEntered` (`self.Driver`) (delegate `Delegate_OnSeatEntered_Event_0`))
  (add `VehicleSeatComponent.Delegate_OnSeatEntered` (`self.VehicleSeat`) (delegate `Delegate_OnSeatEntered_Event_0`)))

(event `Delegate_OnSeatEntered_Event_0`
  (params (Character :type "INSCharacter Object Reference") (Seat :type "VehicleSeatComponent Object Reference")))

(fn `InitMountedGunGameLogic`
  ;[1 1 1] Comment
  (`/Engine/EditorBlueprintResources/ActorMacros.Switch Has Authority`
    (:`Authority`
      (bind _returnvalue (`WeaponStatics.SpawnMountedWeapon` "/Game/Game/Actors/Weapons/Explosive/BP_Explosive_ApacheRockets.BP_Explosive_ApacheRockets_C" self (`self.TurretYaw`) "pitch" (`self.TurretGunner`)))
      (`ItemFirearm.SetFiremode` _returnvalue "Automatic")
      ;;[1 1 1] [Saber Atai] SS-36261- added replication
      (set `self.SpawnedMountedWeapon` _returnvalue)
      (`self.InitMountedGunVisualLogic`))))

(fn `InitMountedGunGameLogic2`
  ;[1 1 1] Comment
  (`/Engine/EditorBlueprintResources/ActorMacros.Switch Has Authority`
    (:`Authority`
      (bind _returnvalue (`WeaponStatics.SpawnMountedWeapon` "/Game/Game/Actors/Weapons/Explosive/BP_Explosive_ApacheRockets.BP_Explosive_ApacheRockets_C" self (`self.TurretYaw`) "pitch" (`self.TurretGunner`)))
      (`ItemFirearm.SetFiremode` _returnvalue "Automatic")
      ;;[1 1 1] [Saber Atai] SS-36261- added replication
      (set `self.SpawnedMountedWeapon` _returnvalue)
      (`self.InitMountedGunVisualLogic`))))

(fn `UserConstructionScript`
  (`parent.UserConstructionScript`))